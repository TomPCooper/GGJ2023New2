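; Main player controller that runs the game's start menu, pause menu and death/respawn flow for Char_Main.
; On begin play it creates the widgets, shows the main menu with ambient sound and disables character input until start.
; BP_DeathCol's death dispatcher triggers rope snapping and the death screen; respawn broadcasts an event and teleports to the latest checkpoint.
; Escape pauses the game; the death screen fade timeline is never run.
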(event Custom|PlayerDeath
  (bind _deathscreen (Variables|Default|GetDeathScreen))
  (Default|RopeSnapping (Variables|Default|GetCharacterRef))
  (Class|BPIUIMenu|IResetStartMenu(Message) _deathscreen)
  (UserInterface|Viewport|AddtoViewport _deathscreen 0)
  (Input|DisableInput (Variables|Default|GetCharacterRef) self))

(event EventICloseMenu
  (Widget|RemovefromParent (Variables|Default|GetPauseMenu))
  (Game|SetGamePaused false))

(event EventIStartGame
  (Widget|RemovefromParent (Variables|Default|GetMainMenu))
  (Game|SetGamePaused false)
  (Input|EnableInput (Variables|Default|GetCharacterRef) self)
  (Audio|Components|Audio|FadeOut (Variables|Default|GetMenuSound) 4.0 0.0 "Linear" :!class /Script/Engine.AudioComponent))

(event EventBeginPlay
  (bind _self self)
  (bind _aschar_main (Utilities|Casting|CastToChar_Main (Pawn|GetControlledPawn)))
  (Variables|Default|SetCharacterRef _aschar_main)
  (bind _returnvalue (UserInterface|CreateWidget "/Game/Core/UI/UI_Menu.UI_Menu_C" _self))
  (Variables|Default|SetMainMenu _returnvalue)
  (bind _returnvalue_2 (UserInterface|CreateWidget "/Game/Core/UI/UI_PauseMenu.UI_PauseMenu_C" _self))
  (Variables|Default|SetPauseMenu _returnvalue_2)
  (Input|DisableInput (Variables|Default|GetCharacterRef) self)
  (UserInterface|Viewport|AddtoViewport (Variables|Default|GetMainMenu) 0)
  (Input|SetInputModeGameandUI self (Variables|Default|GetMainMenu) "DoNotLock" true)
  (bind _returnvalue_3 (Audio|SpawnSound2D "/Game/Core/Audio/Ambience/Summer-Nature-Bird-Sounds.Summer-Nature-Bird-Sounds" 0.6 1.0 0.0 0))
  (Variables|Default|SetMenuSound _returnvalue_3)
  (Variables|Default|SetCurrentRespawn (Transformation|GetActorLocation (Variables|Default|GetCharacterRef)))
  (bind _returnvalue_4 (UserInterface|CreateWidget "/Game/Core/UI/UI_DeathScreen.UI_DeathScreen_C" self))
  (Variables|Default|SetDeathScreen _returnvalue_4)
  (bind _outactors (Actor|GetAllActorsOfClass "/Game/Core/Blueprints/Death/BP_DeathCol.BP_DeathCol_C"))
  (EventDispatchers|BindEventtoEDPlayerDeath _outactors (EventDispatchers|CreateEvent :!event Custom|PlayerDeath)))

(event EventINewCheckpoint
  (params (Checkpoint :type Vector :default "0, 0, 0"))
  (Variables|Default|SetCurrentRespawn Checkpoint))

(event EventIRespawn
  (Widget|RemovefromParent (Variables|Default|GetDeathScreen))
  (Default|CallEDPlayerRespawn)
  (Transformation|SetActorLocation (Variables|Default|GetCharacterRef) (Variables|Default|GetCurrentRespawn) false false)
  (Input|EnableInput (Variables|Default|GetCharacterRef) self))

(event Input|KeyboardEvents|Escape
  (params (Key :type Key%20Structure :default "None"))
  (:Pressed
    (UserInterface|Viewport|AddtoViewport (Variables|Default|GetPauseMenu) 0)
    (Game|SetGamePaused true)))

(fn ConstructionScript)