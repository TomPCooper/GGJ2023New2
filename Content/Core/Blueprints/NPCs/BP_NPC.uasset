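; BP_NPC is an NPC Blueprint with a configurable sprite and a speech bubble that can be shown or hidden.
; The construction script applies TargetSprite to the PaperSprite component, and BeginPlay writes the Speech value into the W_SpeechBubble widget.
; IAddSpeechBubble and IRemoveSpeechBubble events toggle the SpeechBubble component's visibility.
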(event EventIRemoveSpeechBubble
  (Rendering|SetVisibility (Variables|Default|GetSpeechBubble) false false))

(event EventBeginPlay
  (bind _asw_speech_bubble (Utilities|Casting|CastToW_SpeechBubble (UserInterface|GetUserWidgetObject (Variables|Default|GetSpeechBubble))))
  (Default|UpdateText _asw_speech_bubble (Variables|Default|GetSpeech)))

(event EventIAddSpeechBubble
  (Rendering|SetVisibility (Variables|Default|GetSpeechBubble) true false))

(fn ConstructionScript
  (Rendering|Components|Sprite|SetSprite (Variables|Default|GetPaperSprite) (Variables|Default|GetTargetSprite)))