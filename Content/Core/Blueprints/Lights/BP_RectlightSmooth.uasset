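; BP_RectlightSmooth is a rect light whose brightness is animated by a Glow timeline during play.
; The construction script applies TargetLightColour to the light.
; On BeginPlay it caches the light's authored intensity, then plays the timeline and scales that base by the Glow curve on each update.
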(event EventBeginPlay
  (Variables|Default|SetBaseIntensity (Variables|/Script/Engine.LightComponentBase|GetIntensity (Variables|Default|GetRectLight)))
  (bind _glow (Timeline|Glow Play)
    (:Update
      (Rendering|Components|Light|SetIntensity (Variables|Default|GetRectLight) (* _glow (Variables|Default|GetBaseIntensity))))))

(fn ConstructionScript
  (Rendering|Components|Light|SetLightColor (Variables|Default|GetRectLight) (Variables|Default|GetTargetLightColour) true))